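; Player character base with Enhanced Input movement, mouse-style look, launch-based jumping and single-weapon handling.
; Tick rolls the camera from local sideways velocity for strafe tilt, and landing plays a timeline easing roll toward zero.
; Interact attaches the first overlapping BP_WeaponBase to an arrow component, or throws the held one along camera forward with physics enabled.
; Shoot input forwards trigger press and release to the held weapon.
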(event `self.ReceiveBeginPlay`
  (bind _asplayer_controller (cast `PlayerController` (`self.GetController`)))
  (`EnhancedInputSubsystemInterface.AddMappingContext` (pcsubsystem `EnhancedInputLocalPlayerSubsystem` _asplayer_controller) "/Game/BP/Input/IMC_GameplayInput.IMC_GameplayInput" 0 (struct)))

(event `EnhancedInput|/Game/BP/Input/IA_GroundMovement`
  (params (ActionValue :type "Vector2D Structure") (ElapsedSeconds :type "Float (double-precision)") (TriggeredSeconds :type "Float (double-precision)") (InputAction :type "InputAction Object Reference" :default "/Game/BP/Input/IA_GroundMovement.IA_GroundMovement"))
  (bind _arrow1 (`self.Arrow1`))
  (:`Triggered`
    (`self.AddMovementInput` (`SceneComponent.GetForwardVector` _arrow1) ActionValue_X)
    (`self.AddMovementInput` (`SceneComponent.GetRightVector` _arrow1) ActionValue_Y)))

(event `EnhancedInput|/Game/BP/Input/IA_CamLook`
  (params (ActionValue :type "Vector2D Structure") (ElapsedSeconds :type "Float (double-precision)") (TriggeredSeconds :type "Float (double-precision)") (InputAction :type "InputAction Object Reference" :default "/Game/BP/Input/IA_CamLook.IA_CamLook"))
  (:`Triggered`
    (`self.AddControllerPitchInput` (* ActionValue_Y -1.0))
    (`self.AddControllerYawInput` ActionValue_X)))

(event `EnhancedInput|/Game/BP/Input/IA_Jump`
  (params (ActionValue :type Boolean) (ElapsedSeconds :type "Float (double-precision)") (TriggeredSeconds :type "Float (double-precision)") (InputAction :type "InputAction Object Reference" :default "/Game/BP/Input/IA_Jump.IA_Jump"))
  (:`Started`
    (`/Engine/EditorBlueprintResources/StandardMacros.DoOnce` false :!label _label
      (:`Completed`
        (`self.LaunchCharacter` (* (`KismetMathLibrary.Vector_Up`) (`self.JumpVelocity`) (`self.JumpMultiplier`))))))
  (:`Completed`
    (goto _label :!via `Reset`)))

(event `self.ReceiveTick`
  (params (DeltaSeconds :type "Float (single-precision)"))
  (bind _cameramaxtilt (`self.CameraMaxTilt`))
  (bind (_localvelocity_x _localvelocity_y) (`KismetMathLibrary.BreakVector` (`self.LocalVelocity` self)))
  (`SceneComponent.K2_SetRelativeRotation` (`self.Camera`) (`KismetMathLibrary.MakeRotator` (`KismetMathLibrary.MapRangeClamped` _localvelocity_y 600.0 -600.0 _cameramaxtilt (* _cameramaxtilt -1.0))) false false))

(event `FloorCheckLerp`
  (bind _camera (`self.Camera`))
  (bind (_relativerotation_roll _relativerotation_pitch _relativerotation_yaw) (`KismetMathLibrary.BreakRotator` (`SceneComponent.RelativeRotation` _camera)))
  (set `self.PrevRoll` _relativerotation_roll)
  (bind (_direction _lerp) (`Timeline|ReturnToZero` :!via `PlayFromStart`)
    (:`Update`
      (`SceneComponent.K2_SetRelativeRotation` _camera (`KismetMathLibrary.MakeRotator` (`KismetMathLibrary.Lerp` (`self.PrevRoll`) 0.0 _lerp) _relativerotation_pitch _relativerotation_yaw) false false))))

(event `self.OnLanded`
  (params (Hit :type "HitResult Structure (by ref)"))
  (`self.FloorCheckLerp`))

(event `EnhancedInput|/Game/BP/Input/IA_Interact`
  (params (ActionValue :type Boolean) (ElapsedSeconds :type "Float (double-precision)") (TriggeredSeconds :type "Float (double-precision)") (InputAction :type "InputAction Object Reference" :default "/Game/BP/Input/IA_Interact.IA_Interact"))
  (bind _heldweapon (`self.HeldWeapon`))
  (bind _heldweapon_2 (`self.HeldWeapon`))
  (:`Started`
    (`/Engine/EditorBlueprintResources/StandardMacros.IsValid` _heldweapon_2
      (:`Is Valid`
        (`self.K2_DetachFromActor` _heldweapon_2 "KeepWorld" "KeepWorld" "KeepWorld")
        (`/Game/BP/BP_WeaponBase.SetPhysicsState` _heldweapon_2 true)
        (`PrimitiveComponent.AddForce` (`/Game/BP/BP_WeaponBase.r` _heldweapon_2) (* (`SceneComponent.GetForwardVector` (`self.Camera`)) (`self.WeaponThrowForce`)) "None" false))
      (:`Is Not Valid`
        (for _array_element (`PrimitiveComponent.GetOverlappingActors` (`self.Interaction Zone`) "/Game/BP/BP_WeaponBase.BP_WeaponBase_C")
          (set `self.HeldWeapon` (cast `/Game/BP/BP_WeaponBase` _array_element :!pure true))
          (break))
        (`self.K2_AttachToComponent` _heldweapon (`self.Arrow1`) "None" "SnapToTarget" "SnapToTarget" "KeepRelative" true)
        (`/Game/BP/BP_WeaponBase.SetPhysicsState` _heldweapon false)))))

(event `EnhancedInput|/Game/BP/Input/IA_Shoot`
  (params (ActionValue :type Boolean) (ElapsedSeconds :type "Float (double-precision)") (TriggeredSeconds :type "Float (double-precision)") (InputAction :type "InputAction Object Reference" :default "/Game/BP/Input/IA_Shoot.IA_Shoot"))
  (bind _heldweapon (`self.HeldWeapon`))
  (:`Started`
    (`/Game/BP/BP_WeaponBase.PullTrigger` _heldweapon))
  (:`Completed`
    (`/Game/BP/BP_WeaponBase.ReleaseTrigger` _heldweapon)))

(fn `LocalVelocity`
  (params (Target :type "Actor Object Reference"))
  (returns (LocalVelocity :type "Vector Structure"))
  (return (`KismetMathLibrary.InverseTransformDirection` (`self.GetTransform` Target) (`self.GetVelocity` Target))))

(fn `UserConstructionScript`)